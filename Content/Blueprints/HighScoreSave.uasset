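; High score table that holds the top five scores and tracks the current score's rank.
; Check Score bubbles a qualifying score up from fifth place, shifting beaten entries down and recording its position in CurrentScore.
; Later checks from ranks two to five resume at the next higher slot, updating values only on promotion.
; ResetCurrent clears the rank, and GetScores returns the table as one labeled string.
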(fn `Check Score`
  (params (score :type Integer64))
  (switch `int` (`self.currentScore`)
    (:`Default`
      (if (> score (`self.fifth`))
        (set `self.fifth` score)
        (set `self.currentScore` 5)
        (if (> score (`self.fourth`)) :!label _label
          (set `self.fifth` (`self.fourth`))
          (set `self.fourth` score)
          (set `self.currentScore` 4)
          (if (> score (`self.third`)) :!label _label_2
            (set `self.fourth` (`self.third`))
            (set `self.third` score)
            (set `self.currentScore` 3)
            (if (> score (`self.second`)) :!label _label_3
              (set `self.third` (`self.second`))
              (set `self.second` score)
              (set `self.currentScore` 2)
              (if (> score (`self.first`)) :!label _label_4
                (set `self.second` (`self.first`))
                (set `self.first` score)
                (set `self.currentScore` 1)))))))
    (:`2`
      (goto _label_4))
    (:`3`
      (goto _label_3))
    (:`4`
      (goto _label_2))
    (:`5`
      (goto _label))))

(fn `Get Scores`
  (returns (text :type String))
  (return (`KismetStringLibrary.Concat_StrStr` "1st: " (`KismetStringLibrary.Conv_Int64ToString` (`self.first`)) " \n2nd: " (`KismetStringLibrary.Conv_Int64ToString` (`self.second`)) " \n3rd: " (`KismetStringLibrary.Conv_Int64ToString` (`self.third`)) " \n4th: " (`KismetStringLibrary.Conv_Int64ToString` (`self.fourth`)) " \n5th: " (`KismetStringLibrary.Conv_Int64ToString` (`self.fifth`)))))

(fn `ResetCurrent`
  (set `self.currentScore` 0))