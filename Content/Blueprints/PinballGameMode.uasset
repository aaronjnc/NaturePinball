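; Game mode for a pinball game that manages score, lives, balls in play, pausing and game over.
; On BeginPlay it creates the score, game-over and pause widgets, binds start, pause, menu and quit dispatchers, then starts the game.
; Losing the last ball costs a life and respawns through BP_PaddleManager, or shows game over when no lives remain.
; Multiball logic only adjusts counters and never spawns extra balls itself.
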(event `self.ReceiveBeginPlay`
  (`KismetSystemLibrary.PrintString` "Starting game")
  (bind _returnvalue (`|CreateWidget` "/Game/Blueprints/ScoreUI.ScoreUI_C"))
  (bind _output_get (set `self.Score UI` _returnvalue))
  (`UserWidget.AddToViewport` _output_get 0)
  (`self.DisplayScore` 0)
  (bind _returnvalue_2 (`|CreateWidget` "/Game/Blueprints/GameOver.GameOver_C"))
  (bind _output_get_2 (set `self.Game Over UI` _returnvalue_2))
  (`UserWidget.AddToViewport` _output_get_2 2)
  (`Widget.SetVisibility` _output_get_2 "Visible")
  (set `/Game/Blueprints/GameOver.GameMode` self _output_get_2)
  (bind _returnvalue_3 (`|CreateWidget` "/Game/Blueprints/PauseMenu.PauseMenu_C"))
  (bind _output_get_3 (set `self.Pause UI` _returnvalue_3))
  (`UserWidget.AddToViewport` _output_get_3 1)
  (`Widget.SetVisibility` _output_get_3 "Visible")
  (set `/Game/Blueprints/PauseMenu.GameMode` self _output_get_3)
  (add `self.StartDispatcher` (delegate `StartGame`))
  (add `self.PauseDispatcher` (delegate `TogglePause`))
  (add `self.MenuDispatcher` (delegate `Quit to Menu`))
  (add `self.QuitDispatcher` (delegate `Quit Game`))
  (`self.StartDispatcher`)
  (`KismetSystemLibrary.PrintString` "game start complete"))

(event `TogglePause`
  (bind _pause_ui (`self.Pause UI`))
  (`KismetSystemLibrary.PrintString` "Pause input detected")
  (bind _output_get (set `self.paused` (not (`self.paused`))))
  (bind _returnvalue (`GameplayStatics.SetGamePaused` _output_get))
  (if _returnvalue
    (`Widget.SetVisibility` _pause_ui "Visible")
    (else
      (`Widget.SetVisibility` _pause_ui "Hidden"))))

(event `StartGame`
  (`self.ResetGame`))

(event `Quit to Menu`
  (`self.HideAll`)
  (`GameplayStatics.OpenLevel` "Main"))

(event `Quit Game`
  (`KismetSystemLibrary.QuitGame` null "Quit"))

(fn `AddMultiBall`
  (bind _numballsinplay (`self.numBallsInPlay`))
  (`/Engine/EditorBlueprintResources/StandardMacros.DecrementInt` _numballsinplay
    (:`  `
      (`KismetSystemLibrary.PrintString` (`KismetStringLibrary.Conv_IntToString` _numballsinplay))
      (bind _lastball (`self.IsLastBall`))
      (if _lastball
        (`self.SpawnNewBall`)))))

(fn `AddScore`
  (params (Score :type Integer))
  (`self.SetScore` (`KismetMathLibrary.Conv_Int64ToInt` (+ Score (`self.Score`)))))

(fn `DisplayScore`
  (params (NewScore :type Integer64))
  (bind _returnvalue (`KismetTextLibrary.Conv_StringToText` (`KismetStringLibrary.Concat_StrStr` "Score: " (`KismetStringLibrary.Conv_Int64ToString` NewScore))))
  (`TextBlock.SetText` (`/Game/Blueprints/ScoreUI.scoretext` (`self.Score UI`)) _returnvalue)
  (`KismetSystemLibrary.PrintString` (`KismetTextLibrary.Conv_TextToString` _returnvalue)))

(fn `FreeMultiBall`
  (set `self.numBallsInPlay` (+ (`self.multiballCount`) (`self.numBallsInPlay`)))
  (for _ (range (`self.multiballCount`) 1)
    (`self.SpawnMultiBall`))
  (`self.ResetMultiBall`))

(fn `GameOver`
  (`Widget.SetVisibility` (`self.Game Over UI`) "Visible"))

(fn `HideAll`
  (`Widget.SetVisibility` (`self.Game Over UI`) "Hidden")
  (`Widget.SetVisibility` (`self.Score UI`) "Hidden")
  (`Widget.SetVisibility` (`self.Pause UI`) "Hidden"))

(fn `IsLastBall`
  (returns (LastBall :type Boolean))
  (return (== (`self.numBallsInPlay`) 0)))

(fn `LoseBall`
  (`/Engine/EditorBlueprintResources/StandardMacros.DecrementInt` (`self.numBallsInPlay`)
    (:`  `
      (bind _lastball (`self.IsLastBall`))
      (if _lastball
        (if (> (`self.lives`) 0)
          (`self.RemoveLife`)
          (`self.SpawnNewBall`)
          (else
            (`self.GameOver`)
            (`GameplayStatics.PlaySound2D` "/Game/Sounds/gameover.gameover" 1.0 1.0 0.0 null null)))))))

(fn `RemoveLife`
  (set `self.lives` (- (`self.lives`) 1))
  (`GameplayStatics.PlaySound2D` (`self.LostBall`) 1.0 1.0 0.0 null null))

(fn `ResetGame`
  (`self.ResetScore`)
  (`self.ResetMultiBall`)
  (`self.ResetLives`)
  (set `self.numBallsInPlay` 0)
  (set `self.paused` false)
  (`Widget.SetVisibility` (`self.Game Over UI`) "Hidden")
  (`Widget.SetVisibility` (`self.Pause UI`) "Hidden")
  (`self.SpawnNewBall`))

(fn `ResetLives`
  (set `self.lives` (`self.maxLives`)))

(fn `ResetMultiBall`
  (set `self.multiballCount` 0))

(fn `ResetScore`
  (`self.SetScore` (`KismetMathLibrary.Conv_Int64ToInt` 0)))

(fn `SetLives`
  (params (lives :type Integer))
  (set `self.lives` lives))

(fn `SetScore`
  (params (scpre :type Integer))
  (bind _output_get (set `self.Score` (`KismetMathLibrary.Conv_IntToInt64` scpre)))
  (`self.DisplayScore` _output_get))

(fn `SpawnMultiBall`
  (`/Engine/EditorBlueprintResources/StandardMacros.IncrementInt` (`self.numBallsInPlay`)))

(fn `SpawnNewBall`
  (bind _asbp_paddle_manager (cast `/Game/Blueprints/BP_PaddleManager` (`GameplayStatics.GetPlayerPawn` 0)))
  (`/Engine/EditorBlueprintResources/StandardMacros.IncrementInt` (`self.numBallsInPlay`)
    (:`  `
      (`PaddleManager.SpawnBall` _asbp_paddle_manager))))

(fn `UserConstructionScript`)