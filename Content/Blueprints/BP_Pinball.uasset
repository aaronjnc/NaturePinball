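; BP_Pinball is the pinball actor and handles the ball's rolling and impact audio.
; RollSound starts on BeginPlay and replays each time it finishes, with its volume rescaled from the ball's current speed.
; Mushroom hits always play boing and points sounds, while other hits need a strong impulse to play a paddle or wall sound, chosen by casting the other actor.
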(event `self.RollSound.OnAudioFinished`
  (bind _rollsound (`self.RollSound`))
  (`AudioComponent.SetVolumeMultiplier` _rollsound (/ (`KismetMathLibrary.VSize` (`self.GetVelocity`)) 1000.0))
  (`AudioComponent.Play` _rollsound 0.0))

(event `self.Ball.OnComponentHit`
  (params (HitComponent :type "PrimitiveComponent Object Reference") (OtherActor :type "Actor Object Reference") (OtherComp :type "PrimitiveComponent Object Reference") (NormalImpulse :type "Vector Structure") (Hit :type "HitResult Structure (by ref)"))
  (cast `/Game/Blueprints/BP_Mushroom` OtherActor
    (:`then`
      (`GameplayStatics.PlaySound2D` "/Game/Sounds/mushroomboing.mushroomboing" 1.0 1.0 0.0 null null)
      (`GameplayStatics.PlaySound2D` "/Game/Sounds/points_points-St.points_points-St" 1.0 1.0 0.0 null null))
    (:`CastFailed`
      (if (> (`KismetMathLibrary.VSize` NormalImpulse) 5000000.0)
        (cast `/Game/Blueprints/BP_PaddleManager` OtherActor
          (:`then`
            (`GameplayStatics.PlaySound2D` "/Game/Sounds/ballhittingpaddle.ballhittingpaddle" 1.0 1.0 0.0 null null))
          (:`CastFailed`
            (`GameplayStatics.PlaySound2D` "/Game/Sounds/ballhittingwall.ballhittingwall" 1.0 1.0 0.0 null null)))))))

(event `self.ReceiveBeginPlay`
  (`AudioComponent.Play` (`self.RollSound`) 0.0))

(fn `UserConstructionScript`)