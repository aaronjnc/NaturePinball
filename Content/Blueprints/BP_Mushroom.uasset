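; BP_Mushroom is a pinball bumper that pushes the ball on contact and awards points.
; On hit, it applies force to the Pinball along the hit's normal impulse, scaled by Impulse, and adds Score through the cached PinballGameMode.
; The hit also pops the Mushroom component up in scale, and Tick shrinks it linearly back to about normal size.
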(event `self.ReceiveBeginPlay`
  (bind _aspinball_game_mode (cast `/Game/Blueprints/PinballGameMode` (`GameplayStatics.GetGameMode`)))
  (set `self.PinballGameMode` _aspinball_game_mode))

(event `self.ReceiveHit`
  (params (MyComp :type "PrimitiveComponent Object Reference") (Other :type "Actor Object Reference") (OtherComp :type "PrimitiveComponent Object Reference") (bSelfMoved :type Boolean) (HitLocation :type "Vector Structure") (HitNormal :type "Vector Structure") (NormalImpulse :type "Vector Structure") (Hit :type "HitResult Structure (by ref)"))
  (bind _aspinball (cast `Pinball` Other))
  (`Pinball.AddForce` _aspinball (* NormalImpulse (`self.Impulse`)))
  (bind _output_get (set `self.Size` 1.2))
  (`SceneComponent.SetRelativeScale3D` (`self.Mushroom`) (`KismetMathLibrary.Conv_DoubleToVector` _output_get))
  (set `self.IsShrinking` true)
  (`/Game/Blueprints/PinballGameMode.AddScore` (`self.PinballGameMode`) (`self.Score`)))

(event `self.ReceiveTick`
  (params (DeltaSeconds :type "Float (single-precision)"))
  (if (`self.IsShrinking`)
    (bind _output_get (set `self.Size` (- (`self.Size`) (* 0.1 DeltaSeconds))))
    (`SceneComponent.SetRelativeScale3D` (`self.Mushroom`) (`KismetMathLibrary.Conv_DoubleToVector` _output_get))
    (set `self.IsShrinking` (<= 1.0 (`self.Size`)))))

(fn `UserConstructionScript`)