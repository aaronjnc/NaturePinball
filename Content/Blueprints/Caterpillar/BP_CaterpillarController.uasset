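; Caterpillar actor that crawls across the level and destroys itself once it passes a fixed world X limit.
; Each Tick teleports it along its right vector at Speed, without sweeping.
; The same Tick stretches and squashes the root's Y scale at Rate, with the IsIncreasing flag flipping at upper and lower bounds to produce an inching motion.
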(event `self.ReceiveTick`
  (params (DeltaSeconds :type "Float (single-precision)"))
  (bind _returnvalue (`self.GetActorRelativeScale3D`))
  (bind _defaultsceneroot (`self.DefaultSceneRoot`))
  (bind _y (.y _returnvalue))
  (bind _returnvalue_2 (* (`KismetMathLibrary.GetRightVector` (struct)) (* (`self.Rate`) DeltaSeconds)))
  (if (> (`KismetMathLibrary.BreakVector3f` (`self.K2_GetActorLocation`)) 1150.0)
    (`self.K2_DestroyActor`)
    (else
      (`self.K2_SetActorLocation` (+ (* (`self.GetActorRightVector`) (* (`self.Speed`) DeltaSeconds)) (`self.K2_GetActorLocation`)) false true)
      (if (`self.IsIncreasing`)
        (`SceneComponent.SetRelativeScale3D` _defaultsceneroot (+ _returnvalue _returnvalue_2))
        (set `self.IsIncreasing` (<= _y 0.6))
        (else
          (`SceneComponent.SetRelativeScale3D` _defaultsceneroot (- _returnvalue _returnvalue_2))
          (set `self.IsIncreasing` (<= _y 0.45)))))))

(fn `UserConstructionScript`)